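; TrueCreep is an AI character that walks a numbered route of CreepPoint waypoints.
; Its construction script gathers every CreepPoint and sets the initial movement state.
; Each Tick finds the point whose label matches the current index, applies walk speed, calls SimpleMoveToLocation and increments the index within an activation radius, resetting once it exceeds the list length.
; An observe state is only stubbed, and its setter is never executed.
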(event EventTick
  (params (DeltaSeconds :type Float%20%28single-precision%29))
  (bind _currentstate (Variables|Default|GetCurrentState))
  (bind _waypointlist (Variables|Default|GetWaypointList))
  ;[1 1 1] Logic Engine
  (if (Utilities|Enum|Equal(Enum) _currentstate "NewEnumerator0")
    ;[1 1 1] Reset index if needed
    (if (> (Variables|Default|GetTargetCreepPosHolder) (Utilities|Array|Length _waypointlist))
      (Variables|Default|SetTargetCreepPosHolder 0))
    (bind _array_element (Utilities|Array|ForEachLoopwithBreak _waypointlist :!label _label)
      (:LoopBody
        (bind _ascreeppoint_c (Utilities|Casting|CastToCreepPoint _array_element))
        ;[1 1 1] find target waypoint from list of all pertinent waypoints
        (if (== (Variables|/Game/Blueprints/CreepPoint.CreepPoint_C|GetLabelInt _ascreeppoint_c) (Variables|Default|GetTargetCreepPosHolder))
          ;[1 1 1] Grab the Target and its position
          (Variables|Default|SetTargetWaypointPosVec (Transformation|GetActorLocation _ascreeppoint_c))
          (Variables|Default|SetTargetActor _ascreeppoint_c)
          (goto _label Break)))
      (:Completed
        ;[1 1 1] Set Movement Speed
        (Variables|/Script/Engine.CharacterMovementComponent|SetMaxWalkSpeed (Variables|Character|GetCharacterMovement) (* (Variables|Default|GetSpeedRate) (Variables|Default|GetSpeedVariable)))
        ;[1 1 1] Move to Targeted Waypoint
        (AI|Navigation|SimpleMovetoLocation (Pawn|GetController) (Variables|Default|GetTargetWaypointPosVec))
        ;[1 1 1] Check distance from currently targeted Waypoint
        (bind _returnvalue (Transformation|GetDistanceTo (Variables|Default|GetTargetActor)))
        (if (<= _returnvalue (Variables|Default|GetWaypointActivationRadius))
          ;[1 1 1] Queue up next Waypoint
          (Variables|Default|SetTargetCreepPosHolder (+ (Variables|Default|GetTargetCreepPosHolder) 1)))))
    (elif (Utilities|Enum|Equal(Enum) _currentstate "NewEnumerator0")
      (Development|PrintString "Observing")
      (elif (Utilities|Enum|Equal(Enum) _currentstate "NewEnumerator0")
        _))))

(fn ConstructionScript
  (bind _outactors (Actor|GetAllActorsOfClass "/Game/Blueprints/CreepPoint.CreepPoint_C"))
  (Variables|Default|SetWaypointList _outactors)
  (Variables|Default|SetCurrentState "NewEnumerator0"))