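; Hopper is a Character that patrols HopperPoint waypoints using a state machine evaluated every Tick.
; The Construction Script gathers all HopperPoint actors and starts it in the Wander state.
; Wander finds the point whose LabelInt matches the current index, re-issues SimpleMoveToLocation each tick, and advances the index within the activation radius.
; Observe then spins it by a per-tick yaw for set rotations before resuming Wander; two other states are empty.
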(event EventTick
  (params (DeltaSeconds :type Float%20%28single-precision%29))
  (bind _rotation (Variables|Default|GetRotation))
  (bind _waypointlist (Variables|Default|GetWaypointList))
  ;[1 1 1] Logic Engine
  (if (Utilities|Enum|Equal(Enum) (Variables|Default|GetCurrentState) "NewEnumerator0")
    ;[1 1 1] Reset index if needed
    (if (> (Variables|Default|GetTargetCreepPosHolder) (Utilities|Array|Length _waypointlist))
      (Variables|Default|SetTargetCreepPosHolder 0))
    (bind _array_element (Utilities|Array|ForEachLoopwithBreak _waypointlist :!label _label)
      (:LoopBody
        (bind _ashopperpoint_c (Utilities|Casting|CastToHopperPoint _array_element))
        ;[1 1 1] find target waypoint from list of all pertinent waypoints
        (if (== (Variables|/Game/Blueprints/HopperPoint.HopperPoint_C|GetLabelInt _ashopperpoint_c) (Variables|Default|GetTargetCreepPosHolder))
          ;[1 1 1] Grab the Target and its position
          (Variables|Default|SetTargetWaypointPosVec (Transformation|GetActorLocation _ashopperpoint_c))
          (Variables|Default|SetTargetActor _ashopperpoint_c)
          (goto _label Break)))
      (:Completed
        ;[1 1 1] Set Movement Speed
        (Variables|/Script/Engine.CharacterMovementComponent|SetMaxWalkSpeed (Variables|Character|GetCharacterMovement) (* (Variables|Default|GetSpeedRate) (Variables|Default|GetSpeedVariable)))
        ;[1 1 1] Move to Targeted Waypoint
        (AI|Navigation|SimpleMovetoLocation (Pawn|GetController) (Variables|Default|GetTargetWaypointPosVec))
        ;[1 1 1] Check distance from currently targeted Waypoint
        (bind _returnvalue (Transformation|GetDistanceTo (Variables|Default|GetTargetActor)))
        (if (<= _returnvalue (Variables|Default|GetWaypointActivationRadius))
          ;[1 1 1] Queue up next Waypoint
          (Variables|Default|SetTargetCreepPosHolder (+ (Variables|Default|GetTargetCreepPosHolder) 1))
          ;[1 1 1] Enter Observe State
          (Variables|Default|SetCurrentState "NewEnumerator1"))))
    (elif (Utilities|Enum|Equal(Enum) (Variables|Default|GetCurrentState) "NewEnumerator1")
      ;[1 1 1] Apply Rotation
      (Transformation|AddActorLocalRotation (Class|KismetMathLibrary|MakeRot 0.0 _rotation 0.0) false)
      ;[1 1 1] Check if Transition to Wander
      (Variables|Default|SetTotalRotation (+ _rotation (Variables|Default|GetTotalRotation)))
      (if (>= (Variables|Default|GetTotalRotation) (* 3.6e+02 (Variables|Default|GetNumRotationsAllowed)))
        ;[1 1 1] Change State to Wander
        (Variables|Default|SetTotalRotation 0.0)
        (Variables|Default|SetCurrentState "NewEnumerator0"))
      (elif (not (Utilities|Enum|Equal(Enum) (Variables|Default|GetCurrentState) "NewEnumerator3"))
        (if (Utilities|Enum|Equal(Enum) (Variables|Default|GetCurrentState) "NewEnumerator2")
          _)))))

(fn ConstructionScript
  (bind _outactors (Actor|GetAllActorsOfClass "/Game/Blueprints/HopperPoint.HopperPoint_C"))
  (Variables|Default|SetWaypointList _outactors)
  (Variables|Default|SetCurrentState "NewEnumerator0"))